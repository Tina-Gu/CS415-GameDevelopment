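; Enemy actor that reacts to overlaps on its Cube component with projectiles and the player.
; A Projectile overlap destroys the enemy and adds a fixed bonus to the player pawn's Score.
; A BP_Player overlap instead subtracts CurrentHealth and starts a screen camera shake through the player's CameraShakeSource, leaving the enemy in place.
; It has no movement or tick logic of its own.
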(event OnComponentBeginOverlap(Cube)
  (params (OverlappedComponent :type Primitive%20Component%20Object%20Reference) (OtherActor :type Actor%20Object%20Reference) (OtherComp :type Primitive%20Component%20Object%20Reference) (OtherBodyIndex :type Integer) (bFromSweep :type Boolean) (SweepResult :type Hit%20Result%20Structure%20%28by%20ref%29))
  (Utilities|Casting|CastToProjectile OtherActor
    (:then
      (Actor|DestroyActor)
      (bind _asbp_player (Utilities|Casting|CastToBP_Player (Game|Player|GetPlayerPawn 0)))
      (Variables|/Game/InfiniteMatrix/Blueprints/BP_Player.BP_Player_C|SetScore _asbp_player (+ (Variables|/Game/InfiniteMatrix/Blueprints/BP_Player.BP_Player_C|GetScore _asbp_player) 3e+01)))
    (:CastFailed
      (bind _asbp_player_2 (Utilities|Casting|CastToBP_Player OtherActor))
      (Variables|/Game/InfiniteMatrix/Blueprints/BP_Player.BP_Player_C|SetCurrentHealth _asbp_player_2 (- (Variables|/Game/InfiniteMatrix/Blueprints/BP_Player.BP_Player_C|GetCurrentHealth _asbp_player_2) 5.0))
      (CameraShakes|StartCameraShake (Variables|/Game/InfiniteMatrix/Blueprints/BP_Player.BP_Player_C|GetCameraShakeSource _asbp_player_2) "/Game/InfiniteMatrix/Blueprints/ScreenShake.ScreenShake_C" 1.0 "CameraLocal" "0, 0, 0"))))

(event EventBeginPlay)

(event Collision|EventActorBeginOverlap
  (params (OtherActor :type Actor%20Object%20Reference)))

(event EventTick
  (params (DeltaSeconds :type Float%20%28single-precision%29)))

(fn ConstructionScript)